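; Sliding door actor that opens when its Interact event fires and reverses after a delay; despite the Locked name, this graph contains no lock check.
; BeginPlay caches the start location, and a timeline drives the offset from it.
; Yaw comparisons against four cardinal angles pick the world axis and sign of the slide, so other angles produce no movement.
; The timeline's Finished output calls DoorOpened, which waits, then reverses the timeline.
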(event `self.ReceiveBeginPlay`
  ;[1 1 1] Original door location init
  (set `self.Door Initial Location` (`self.K2_GetActorLocation` self)))

(event `self.Interact`
  (params (Character :type "CVCharacter Object Reference"))
  (bind _door_initial_location (`self.Door Initial Location`))
  (bind _door_initial_location_2 (`self.Door Initial Location`))
  (bind _yaw (.yaw (`self.K2_GetActorRotation`)))
  ;[1 1 1] Open and close door
  (bind (_direction _door_movement) (`Timeline|Timeline_0` :!label _label)
    (:`Update`
      (if (`KismetMathLibrary.NearlyEqual_FloatFloat` _yaw 0.0 0.1)
        (`self.K2_SetActorRelativeLocation` (+ _door_initial_location_2 (`KismetMathLibrary.MakeVector` _door_movement)))
        (elif (`KismetMathLibrary.NearlyEqual_FloatFloat` _yaw 90.0 0.1)
          (`self.K2_SetActorRelativeLocation` (+ _door_initial_location_2 (`KismetMathLibrary.MakeVector` 0.0 _door_movement)))
          (elif (`KismetMathLibrary.NearlyEqual_FloatFloat` _yaw -180.0 0.1)
            (`self.K2_SetActorRelativeLocation` (- _door_initial_location (`KismetMathLibrary.MakeVector` _door_movement)))
            (elif (`KismetMathLibrary.NearlyEqual_FloatFloat` _yaw -90.0 0.1)
              (`self.K2_SetActorRelativeLocation` (- _door_initial_location (`KismetMathLibrary.MakeVector` 0.0 _door_movement))))))))
    (:`Finished`
      (`self.Door Opened`))))

(event `Door Opened`
  ;[1 1 1] Open and close door
  (`KismetSystemLibrary.Delay` 3.0)
  (goto _label :!via `Reverse`))

(fn `UserConstructionScript`)