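; Bank double sliding door that opens on Interact and is set to reverse closed after a short delay.
; BeginPlay caches both panels' world origins, and a timeline offsets them in opposite directions from there.
; The slide axis and sign are picked by comparing actor yaw to the four cardinal angles, so other rotations leave the panels still.
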(event `self.ReceiveBeginPlay`
  ;[1 1 1] Original door location init
  (set `self.RightDoorOrigin` (`SceneComponent.K2_GetComponentLocation` (`self.RightDoor_F`)))
  (set `self.LeftDoorOrigin` (`SceneComponent.K2_GetComponentLocation` (`self.LeftDoor_F`))))

(event `self.Interact`
  (params (Character :type "CVCharacter Object Reference"))
  (bind _leftdoororigin (`self.LeftDoorOrigin`))
  (bind _rightdoororigin (`self.RightDoorOrigin`))
  (bind _leftdoororigin_2 (`self.LeftDoorOrigin`))
  (bind _rightdoororigin_2 (`self.RightDoorOrigin`))
  (bind _yaw (.yaw (`self.K2_GetActorRotation`)))
  ;[1 1 1] Opening and closing of doors
  (bind (_direction _door_movement) (`Timeline|Timeline_0` :!label _label)
    (:`Update`
      (if (`KismetMathLibrary.NearlyEqual_FloatFloat` _yaw)
        (bind _returnvalue (`KismetMathLibrary.MakeVector` _door_movement))
        (`SceneComponent.K2_SetWorldLocation` (`self.LeftDoor_F`) (- _leftdoororigin _returnvalue) false false)
        (`SceneComponent.K2_SetWorldLocation` (`self.RightDoor_F`) (+ _returnvalue _rightdoororigin) false false)
        (elif (`KismetMathLibrary.NearlyEqual_FloatFloat` _yaw 90.0 0.1)
          (bind _returnvalue_2 (`KismetMathLibrary.MakeVector` 0.0 _door_movement))
          (`SceneComponent.K2_SetWorldLocation` (`self.LeftDoor_F`) (- _leftdoororigin _returnvalue_2) false false)
          (`SceneComponent.K2_SetWorldLocation` (`self.RightDoor_F`) (+ _rightdoororigin _returnvalue_2) false false)
          (elif (`KismetMathLibrary.NearlyEqual_FloatFloat` _yaw -180.0 0.1)
            (bind _returnvalue_3 (`KismetMathLibrary.MakeVector` _door_movement))
            (`SceneComponent.K2_SetWorldLocation` (`self.LeftDoor_F`) (+ _returnvalue_3 _leftdoororigin_2) false false)
            (`SceneComponent.K2_SetWorldLocation` (`self.RightDoor_F`) (- _rightdoororigin_2 _returnvalue_3) false false)
            (elif (`KismetMathLibrary.NearlyEqual_FloatFloat` _yaw -90.0 0.1)
              (bind _returnvalue_4 (`KismetMathLibrary.MakeVector` 0.0 _door_movement))
              (`SceneComponent.K2_SetWorldLocation` (`self.LeftDoor_F`) (+ _leftdoororigin_2 _returnvalue_4) false false)
              (`SceneComponent.K2_SetWorldLocation` (`self.RightDoor_F`) (- _rightdoororigin_2 _returnvalue_4) false false))))))
    (:`Finished`
      (`self.Door Opened`))))

(event `Door Opened`
  ;[1 1 1] Opening and closing of doors
  (`KismetSystemLibrary.Delay` 3.0)
  (goto _label :!via `Reverse`))

(fn `UserConstructionScript`)