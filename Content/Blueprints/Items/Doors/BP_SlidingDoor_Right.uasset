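; BP_SlidingDoor_Right is a sliding door actor that opens on Interact and closes itself after a delay.
; BeginPlay stores the world location, and Timeline_Door adds its DoorMovement value along X to that, applied as relative location.
; The timeline's Finished output calls DoorOpened, which waits three seconds and reverses the timeline, with no check on play direction.
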(event `self.Interact`
  (params (Character :type "CVCharacter Object Reference"))
  ;[1 1 1] Open and close door
  (bind (_direction _door_movement) (`Timeline|Timeline_Door` :!label _label)
    (:`Update`
      (`self.K2_SetActorRelativeLocation` (+ (`self.Door Initial Location`) (`KismetMathLibrary.MakeVector` _door_movement))))
    (:`Finished`
      (`self.Door Opened`))))

(event `Door Opened`
  ;[1 1 1] Open and close door
  (`KismetSystemLibrary.Delay` 3.0)
  (goto _label :!via `Reverse`))

(event `self.ReceiveBeginPlay`
  ;[1 1 1] Original door location init
  (set `self.Door Initial Location` (`self.K2_GetActorLocation` self)))

(fn `UserConstructionScript`)