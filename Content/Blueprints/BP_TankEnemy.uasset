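; BP_TankEnemy is a tank enemy actor driven by an AI controller and a health component.
; ActivateAI runs the BT_TestEnemy behavior tree on its controller, and DeactivateAI stops that controller's brain logic.
; Each health change briefly draws the new value as debug text at the actor's location.
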(event `self.HealthComp.OnHealthChanged`
  (params (HealthComp :type "CVHealthComponent Object Reference") (Health :type "Float (single-precision)") (HealthDelta :type "Float (single-precision)") (DamageType :type "DamageType Object Reference") (InstigatedBy :type "Controller Object Reference") (DamageCauser :type "Actor Object Reference"))
  (`KismetSystemLibrary.DrawDebugString` (`self.K2_GetActorLocation`) (`KismetStringLibrary.Conv_DoubleToString` Health) null (struct :`R` 1.0 :`G` 0.853204 :`A` 1.0) 1.0))

(fn `ActivateAI`
  (`AIController.RunBehaviorTree` (`AIBlueprintHelperLibrary.GetAIController` self) "/Game/Blueprints/AI/BT_TestEnemy.BT_TestEnemy"))

(fn `DeactivateAI`
  (`BrainComponent.StopLogic` (`AIController.BrainComponent` (`AIBlueprintHelperLibrary.GetAIController` self)) ""))

(fn `UserConstructionScript`)