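; Behavior Tree service that picks a target character for an AI pawn.
; Each tick it scans the actors known through the pawn's AIPerception sight sense and takes the first CVCharacter whose CVHealthComponent health is above zero.
; It writes the stored target to a Blackboard key, and that variable is not cleared when no living character is found.
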(event `self.ReceiveTickAI`
  (params (OwnerController :type "AIController Object Reference") (ControlledPawn :type "Pawn Object Reference") (DeltaSeconds :type "Float (single-precision)"))
  (for _array_element (`AIPerceptionComponent.GetKnownPerceivedActors` (`Actor.GetComponentByClass` ControlledPawn "/Script/AIModule.AIPerceptionComponent") "/Script/AIModule.AISense_Sight")
    (bind _ascvcharacter (cast `CVCharacter` _array_element))
    (`/Engine/EditorBlueprintResources/StandardMacros.IsValid` _ascvcharacter
      (:`Is Valid`
        (if (> (`CVHealthComponent.Health` (`Actor.GetComponentByClass` _ascvcharacter "/Script/Cyber_Vitae.CVHealthComponent")) 0.0)
          (set `self.TargetCharacter` _ascvcharacter)
          (break)))))
  (`BTFunctionLibrary.SetBlackboardValueAsObject` (`self.Blackboard Key`) (`self.TargetCharacter`)))